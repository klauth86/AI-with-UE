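; AI controller that reports sight perception changes as on-screen debug text, with no behavior logic.
; On each target perception update from its sight perception component, it prints the actor's name, entered or left, the stimulus's sense class and the perceived actor count.
; Entered or left comes from whether the actor is in the component's perceived actors list, rather than from the stimulus itself.
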(event `self.SightPerceptionComponent.OnTargetPerceptionUpdated`
  (params (Actor :type "Actor Object Reference") (Stimulus :type "AIStimulus Structure"))
  (bind _outactors (`AIPerceptionComponent.GetPerceivedActors` (`self.SightPerceptionComponent`) null))
  (bind _returnvalue (`AIPerceptionSystem.GetSenseClassForStimulus` Stimulus))
  (`KismetSystemLibrary.PrintString` (`KismetStringLibrary.Concat_StrStr` (`KismetSystemLibrary.GetDisplayName` Actor) (`KismetMathLibrary.SelectString` " entered " " left " (`KismetArrayLibrary.Array_Contains` _outactors Actor)) (`KismetSystemLibrary.GetClassDisplayName` _returnvalue) "(" (`KismetStringLibrary.Conv_IntToString` (`KismetArrayLibrary.Array_Length` _outactors)) ")")))

(fn `UserConstructionScript`)