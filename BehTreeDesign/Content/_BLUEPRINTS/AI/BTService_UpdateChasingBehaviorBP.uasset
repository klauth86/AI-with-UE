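; Behavior tree service that keeps the blackboard updated with player-chasing information for an AI.
; On activation it stores the first Player actor found in the level in the player key.
; Each tick it copies the ChasingAIController's CanSeePlayer flag to the blackboard.
; When that flag differs from its cached value, it also writes the controller's last known player position and updates the cache.
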(event `self.ReceiveActivationAI`
  (params (OwnerController :type "AIController Object Reference") (ControlledPawn :type "Pawn Object Reference"))
  (bind _outactors (`GameplayStatics.GetAllActorsOfClass` "/Game/ThirdPersonCPP/Blueprints/Player.Player_C"))
  (`BTFunctionLibrary.SetBlackboardValueAsObject` (`self.PlayerKey`) (`|GetArrayItem` _outactors)))

(event `self.ReceiveTickAI`
  (params (OwnerController :type "AIController Object Reference") (ControlledPawn :type "Pawn Object Reference") (DeltaSeconds :type "Float (single-precision)"))
  (bind _aschasing_aicontroller (cast `ChasingAIController` OwnerController))
  (bind _bcanseeplayer (`ChasingAIController.bCanSeePlayer` _aschasing_aicontroller))
  (`BTFunctionLibrary.SetBlackboardValueAsBool` (`self.CanSeePlayerKey`) _bcanseeplayer)
  (if (not (== _bcanseeplayer (`self.LastCanSeePlayer`)))
    (`BTFunctionLibrary.SetBlackboardValueAsVector` (`self.LastKnownPositionKey`) (`ChasingAIController.LastKnownPlayerPosition` _aschasing_aicontroller))
    (set `self.LastCanSeePlayer` (`BTFunctionLibrary.GetBlackboardValueAsBool` (`self.CanSeePlayerKey`)))))